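; Spawner actor that builds a lane-based crossing level and populates it with vehicles, logs, scenery and coins.
; BeginPlay chains BP_Water tiles from an offset off the player, each at the previous tile's SpawnPoint, starting as grass before randomizing meshes.
; Tiles receive a Spawner reference, and per-type functions spawn props at offsets from a given location, often randomized.
; Log pairs share one speed; car and truck pair branches never run.
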(event `self.ReceiveBeginPlay`
  (`self.SpawnInitialWater`))

(fn `SpawnBus`
  (params (SpawnLocation :type "Vector Structure"))
  (`|SpawnActorFromClass` "/Game/Blueprints/BP_Bus.BP_Bus_C" (`KismetMathLibrary.MakeTransform` (`KismetMathLibrary.MakeVector` (+ SpawnLocation_X 1.0) (+ SpawnLocation_Y 1.0) (+ SpawnLocation_Z 1.0))) "Undefined" "OverrideRootScale" null null))

(fn `SpawnCar`
  (params (SpawnLocation :type "Vector Structure"))
  (if (> 0 60)
    (for _index (range 2)
      (bind _returnvalue (`|SpawnActorFromClass` "/Game/Blueprints/BP_Car.BP_Car_C" (`KismetMathLibrary.MakeTransform` (`KismetMathLibrary.MakeVector` (+ SpawnLocation_X 255.0) (+ (+ SpawnLocation_Y 2200.0) (* _index (`KismetMathLibrary.RandomFloatInRange` 300.0 400.0))) (+ SpawnLocation_Z 5.0))) "Undefined" "OverrideRootScale" null null))
      (if (< _index 1)
        (set `self.NewSpeed` (`/Game/Blueprints/BP_Car.max_speed` _returnvalue))
        (set `/Game/Blueprints/BP_Car.max_speed` (`self.NewSpeed`) _returnvalue)))
    (else
      (`|SpawnActorFromClass` "/Game/Blueprints/BP_Car.BP_Car_C" (`KismetMathLibrary.MakeTransform` (`KismetMathLibrary.MakeVector` (+ SpawnLocation_X 255.0) (+ SpawnLocation_Y 2200.0) (+ SpawnLocation_Z 5.0))) "Undefined" "OverrideRootScale" null null))))

(fn `SpawnCoin`
  (params (SpawnLocation :type "Vector Structure"))
  (for _ (range (+ (`KismetMathLibrary.RandomIntegerInRange` 0 3) 1))
    (`|SpawnActorFromClass` "/Game/Blueprints/BP_Coin.BP_Coin_C" (`KismetMathLibrary.MakeTransform` (`KismetMathLibrary.MakeVector` (+ SpawnLocation_X 340.0) (+ SpawnLocation_Y (`KismetMathLibrary.RandomFloatInRange` 1600.0 4400.0)) (+ SpawnLocation_Z 500.0))) "Undefined" "OverrideRootScale" null null)))

(fn `SpawnInitialWater`
  (for _ (range 26)
    (`/Engine/EditorBlueprintResources/StandardMacros.IsValid` (`self.NewestWater`)
      (:`Is Valid`
        (`self.SpawnWaterAtSpawnPoint`))
      (:`Is Not Valid`
        (`self.SpawnWater` (+ (`self.K2_GetActorLocation` (`GameplayStatics.GetPlayerCharacter` 0)) (`self.StartPoint`)))))))

(fn `SpawnLilyPad`
  (params (SpawnLocation :type "Vector Structure"))
  (bind _returnvalue (`KismetMathLibrary.RandomFloatInRange` 3500.0 4000.0))
  (`|SpawnActorFromClass` "/Game/Blueprints/BP_LilyPad.BP_LilyPad_C" (`KismetMathLibrary.MakeTransform` (`KismetMathLibrary.MakeVector` (+ SpawnLocation_X 110.0) (+ (- SpawnLocation_Y 5.0) (- _returnvalue (mod _returnvalue 120.0))) (+ SpawnLocation_Z 50.0))) "Undefined" "OverrideRootScale" null null))

(fn `SpawnLog`
  (params (SpawnLocation :type "Vector Structure"))
  (for _index (range 2)
    (bind _returnvalue (`|SpawnActorFromClass` "/Game/Blueprints/BP_Log.BP_Log_C" (`KismetMathLibrary.MakeTransform` (`KismetMathLibrary.MakeVector` (- SpawnLocation_X 23.0) (+ (* _index 300.0) (+ SpawnLocation_Y 2200.0)) (+ SpawnLocation_Z 55.0))) "Undefined" "OverrideRootScale" null null))
    (if (< _index 1)
      (set `self.NewSpeed` (`/Game/Blueprints/BP_Log.max_speed` _returnvalue))
      (else
        (set `/Game/Blueprints/BP_Log.max_speed` (`self.NewSpeed`) _returnvalue)))))

(fn `SpawnLongLog`
  (params (SpawnLocation :type "Vector Structure (by ref)"))
  (for _index (range 2)
    (bind _returnvalue (`|SpawnActorFromClass` "/Game/Blueprints/BP_LongLog.BP_LongLog_C" (`KismetMathLibrary.MakeTransform` (`KismetMathLibrary.MakeVector` (- SpawnLocation_X 23.0) (+ (* _index 300.0) (+ SpawnLocation_Y 4500.0)) (+ SpawnLocation_Z 55.0))) "Undefined" "OverrideRootScale" null null))
    (if (< _index 1)
      (set `self.NewSpeed` (`/Game/Blueprints/BP_LongLog.max_speed` _returnvalue))
      (else
        (set `/Game/Blueprints/BP_LongLog.max_speed` (`self.NewSpeed`) _returnvalue)))))

(fn `SpawnRock`
  (params (SpawnLocation :type "Vector Structure"))
  (bind _returnvalue (`KismetMathLibrary.RandomFloatInRange` 1600.0 4400.0))
  (bind _returnvalue_2 (+ (- SpawnLocation_Y 30.0) (- _returnvalue (mod _returnvalue 120.0))))
  (for _ (range (+ (`KismetMathLibrary.RandomIntegerInRange` 1 5) 1))
    (`|SpawnActorFromClass` "/Game/Blueprints/BP_Rock.BP_Rock_C" (`KismetMathLibrary.MakeTransform` (`KismetMathLibrary.MakeVector` (+ SpawnLocation_X 100.0) _returnvalue_2 (+ SpawnLocation_Z 150.0))) "Undefined" "OverrideRootScale" null null)
    (`BlueprintSetLibrary.Set_Add` (`self.RockTrees`) _returnvalue_2)
    (if true
      _)))

(fn `SpawnSmallBush`
  (params (SpawnLocation :type "Vector Structure"))
  (for _ (range (+ (`KismetMathLibrary.RandomIntegerInRange` 0 5) 1))
    (`|SpawnActorFromClass` "/Game/Blueprints/BP_SmallBush.BP_SmallBush_C" (`KismetMathLibrary.MakeTransform` (`KismetMathLibrary.MakeVector` (+ SpawnLocation_X 1.0) (+ SpawnLocation_Y (`KismetMathLibrary.RandomFloatInRange` 1600.0 2400.0)) (+ SpawnLocation_Z 1.0))) "Undefined" "OverrideRootScale" null null)))

(fn `SpawnTrain`
  (params (SpawnLocation :type "Vector Structure"))
  (locals (Train :type "/Game/Blueprints/BP_Train Object Reference"))
  (`|SpawnActorFromClass` "/Game/Blueprints/BP_Train.BP_Train_C" (`KismetMathLibrary.MakeTransform` (`KismetMathLibrary.MakeVector` SpawnLocation_X SpawnLocation_Y (- SpawnLocation_Z 20.0))) "Undefined" "OverrideRootScale" null null))

(fn `SpawnTrainPost`
  (params (SpawnLocation :type "Vector Structure"))
  (`|SpawnActorFromClass` "/Game/Blueprints/BP_TrainPost.BP_TrainPost_C" (`KismetMathLibrary.MakeTransform` (`KismetMathLibrary.MakeVector` (+ SpawnLocation_X 190.0) (+ SpawnLocation_Y 2900.0) (+ SpawnLocation_Z 150.0))) "Undefined" "OverrideRootScale" null null))

(fn `SpawnTrainTracks`
  (params (SpawnLocation :type "Vector Structure"))
  (`|SpawnActorFromClass` "/Game/Blueprints/BP_TrainTracks.BP_TrainTracks_C" (`KismetMathLibrary.MakeTransform` (`KismetMathLibrary.MakeVector` (- SpawnLocation_X 260.0) (+ SpawnLocation_Y 6000.0) (- SpawnLocation_Z 40.0))) "Undefined" "OverrideRootScale" null null))

(fn `SpawnTree`
  (params (SpawnLocation :type "Vector Structure"))
  (bind _returnvalue (`KismetMathLibrary.RandomFloatInRange` 1600.0 4400.0))
  (bind _returnvalue_2 (+ SpawnLocation_Y (- _returnvalue (mod _returnvalue 120.0))))
  (for _ (range (+ (`KismetMathLibrary.RandomIntegerInRange` 0 5) 1))
    (`|SpawnActorFromClass` "/Game/Blueprints/BP_Tree.BP_Tree_C" (`KismetMathLibrary.MakeTransform` (`KismetMathLibrary.MakeVector` (+ SpawnLocation_X 80.0) _returnvalue_2 (+ SpawnLocation_Z 90.0))) "Undefined" "OverrideRootScale" null null)
    (`BlueprintSetLibrary.Set_Add` (`self.RockTrees`) _returnvalue_2)))

(fn `SpawnTruck`
  (params (SpawnLocation :type "Vector Structure"))
  (if (> 0 60)
    (for _index (range 2)
      (bind _returnvalue (`|SpawnActorFromClass` "/Game/Blueprints/BP_Truck.BP_Truck_C" (`KismetMathLibrary.MakeTransform` (`KismetMathLibrary.MakeVector` (- SpawnLocation_X 275.0) (+ (* _index (`KismetMathLibrary.RandomFloatInRange` 300.0 400.0)) (+ SpawnLocation_Y 4200.0)) (+ SpawnLocation_Z 25.0))) "Undefined" "OverrideRootScale" null null))
      (if (< _index 1)
        (set `self.NewSpeed` (`/Game/Blueprints/BP_Truck.max_speed` _returnvalue))
        (else
          (set `/Game/Blueprints/BP_Truck.max_speed` (`self.NewSpeed`) _returnvalue))))
    (else
      (`|SpawnActorFromClass` "/Game/Blueprints/BP_Truck.BP_Truck_C" (`KismetMathLibrary.MakeTransform` (`KismetMathLibrary.MakeVector` (- SpawnLocation_X 275.0) (+ SpawnLocation_Y 4200.0) (+ SpawnLocation_Z 25.0))) "Undefined" "OverrideRootScale" null null))))

(fn `SpawnWater`
  (params (TargetLocation :type "Vector Structure"))
  (set `self.WaterCount` (+ (`self.WaterCount`) 1))
  (bind _returnvalue (`|SpawnActorFromClass` "/Game/Blueprints/BP_Water.BP_Water_C" (`KismetMathLibrary.MakeTransform` TargetLocation) "Undefined" "OverrideRootScale" null null))
  (bind _output_get (set `self.NewestWater` _returnvalue))
  (set `/Game/Blueprints/BP_Water.Spawner` self _output_get)
  (if (> (`self.WaterCount`) 7)
    (`/Game/Blueprints/BP_Water.RandomizeMesh` _output_get)
    (else
      (`/Game/Blueprints/BP_Water.InitialGrass` _output_get))))

(fn `SpawnWaterAtSpawnPoint`
  (`self.SpawnWater` (`SceneComponent.K2_GetComponentLocation` (`/Game/Blueprints/BP_Water.SpawnPoint` (`self.NewestWater`)))))

(fn `SpawnYellowCar`
  (params (SpawnLocation :type "Vector Structure"))
  (`|SpawnActorFromClass` "/Game/Blueprints/BP_YellowCar.BP_YellowCar_C" (`KismetMathLibrary.MakeTransform` (`KismetMathLibrary.MakeVector` (+ SpawnLocation_X 1.0) (+ SpawnLocation_Y 1.0) (+ SpawnLocation_Z 1.0))) "Undefined" "OverrideRootScale" null null))

(fn `UserConstructionScript`)